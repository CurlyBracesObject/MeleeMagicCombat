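; BP_DecalActor is a targeting decal shown while the player prepares to release a skill.
; Each Tick it moves its Decal to the HitLocation of player 0's BP_Character.
; It destroys itself once that character's SkillIndex is no longer 1.
; Logic to spawn BP_DamegedActor at SkillIndex 0 is left unconnected, with a note that the decal is already destroyed by then.
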(event EventTick
  (params (DeltaSeconds :type Float%20%28single-precision%29))
  (bind _returnvalue (Game|GetPlayerCharacter 0))
  (bind _asbp_character (Utilities|Casting|CastToBP_Character _returnvalue))
  (Utilities|FlowControl|Sequence
    (:then_0
      ;[1 1 1] 技能准备释放中 decalacto任意跟随
      (Transformation|SetWorldLocation (Variables|Default|GetDecal) (Variables|/Game/ThirdGame/Character/BP_Character.BP_Character_C|GetHitLocation _asbp_character) false false))
    (:then_1
      (if (not (== (Variables|/Game/ThirdGame/Character/BP_Character.BP_Character_C|GetSkillIndex _asbp_character) 1))
        (Actor|DestroyActor)))))

(event EventBeginPlay
  ;[1 1 1] 不能在tick里写生成emitter特效    in beginplay, skillindex need to be 0 then spawn damaged emitter,but when 0,the decal actor already destroied
)

(fn ConstructionScript)