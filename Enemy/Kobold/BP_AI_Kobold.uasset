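; Kobold enemy character that damages the player.
; A callable event applies damage to player 0, while capsule overlap with a BP_Character applies a separate, slightly smaller hit.
; The construction script makes the modular armor and clothing meshes follow the main mesh through master pose.
; Death montage and animation logic is present but disconnected, so this graph never handles the Kobold's death.
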(event OnComponentBeginOverlap(Capsule)
  (params (OverlappedComponent :type Primitive%20Component%20Object%20Reference) (OtherActor :type Actor%20Object%20Reference) (OtherComp :type Primitive%20Component%20Object%20Reference) (OtherBodyIndex :type Integer) (bFromSweep :type Boolean) (SweepResult :type Hit%20Result%20Structure%20%28by%20ref%29))
  (bind _asbp_character (Utilities|Casting|CastToBP_Character OtherActor))
  (bind _returnvalue (Game|Damage|ApplyDamage _asbp_character 1e+01 0 0)))

(event Custom|ApplayDamtoPlayer
  (bind _returnvalue (Game|Damage|ApplyDamage (Game|GetPlayerCharacter 0) 12.0 0 self))
  (Development|PrintString (Utilities|String|ToString(Float) _returnvalue)))

(event EventBeginPlay
  (|CallParentFunction))

(event EventTick
  (params (DeltaSeconds :type Float%20%28single-precision%29))
  (|CallParentFunction DeltaSeconds))

(fn ConstructionScript
  (Class|SkinnedMeshComponent|SetMasterPoseComponent (Variables|Default|GetSK_KOBOLD_ShoulderPads) (Variables|Character|GetMesh) false))