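; BP_AI is an enemy actor with health, a floating health widget that turns toward the camera, and a death report to the game mode.
; AnyDamage lowers clamped HP, and SetMonsterType sets HP from MonsterIndex.
; Tick detects zero HP while the widget is visible, then once reports the kill and destroys the actor after a delay.
; Older death-animation, blackboard and respawn logic remains unconnected.
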(event Custom|SetMonsterType
  (Utilities|FlowControl|Sequence
    (:then_0
      (if (== (Variables|Default|GetMonsterIndex) 1)
        (Variables|Default|SetCurrentHP 2e+01)
        (Variables|Default|SetMaxHP 2e+01)
        (Development|PrintString "HP20")))
    (:then_1
      (if (== (Variables|Default|GetMonsterIndex) 2)
        (Variables|Default|SetCurrentHP 1e+01)
        (Variables|Default|SetMaxHP 1e+01)
        (Development|PrintString "HP10")))))

(event Custom|AfterAIDie
  (Default|ReportEnemyKilled (.AsBP%20Game%20Mode%20Base (Utilities|Casting|CastToBP_GameModeBase (Game|GetGameMode))))
  (Utilities|FlowControl|Delay 1.8)
  (Rendering|SetVisibility (Variables|Default|GetAIBloodUI) false false)
  (Actor|DestroyActor))

(event EventBeginPlay
  (bind _asbp_aiblood_ui (Utilities|Casting|CastToBP_AIBloodUI (UserInterface|GetUserWidgetObject (Variables|Default|GetAIBloodUI))))
  (Variables|/Game/ThirdGame/UI/BP_AIBloodUI.BP_AIBloodUI_C|SetEnemy _asbp_aiblood_ui self)
  (Variables|/Game/ThirdGame/GameModeBase/BP_GameModeBase.BP_GameModeBase_C|SetAIActor (.AsBP%20Game%20Mode%20Base (Utilities|Casting|CastToBP_GameModeBase (Game|GetGameMode))) self))

(event EventTick
  (params (DeltaSeconds :type Float%20%28single-precision%29))
  (bind _aibloodui (Variables|Default|GetAIBloodUI))
  (if (Rendering|IsVisible _aibloodui)
    (Transformation|SetWorldRotation _aibloodui (Math|Rotator|FindLookatRotation (Transformation|GetWorldLocation _aibloodui) (Transformation|GetActorLocation (Game|GetPlayerCameraManager 0))) false false)
    (Utilities|FlowControl|Sequence
      (:then_0
        (Variables|Default|SetIsDeath (== (Variables|Default|GetCurrentHP) 0.0))
        (if (Variables|Default|GetIsDeath)
          (Utilities|FlowControl|DoOnce false
            (:Completed
              (CallFunction|AfterAIDie))))))))

(event Game|Damage|EventAnyDamage
  (params (Damage :type Float%20%28single-precision%29) (DamageType :type Damage%20Type%20Object%20Reference) (InstigatedBy :type Controller%20Object%20Reference) (DamageCauser :type Actor%20Object%20Reference))
  (Variables|Default|SetCurrentHP (Math|Float|Clamp(Float) (- (Variables|Default|GetCurrentHP) Damage) 0.0 (Variables|Default|GetMaxHP))))

(fn ConstructionScript)

(fn LogicAfterAIDeath)