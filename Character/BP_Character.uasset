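; Player character with axis-driven movement and look, clamped damage to HP, a normal attack and one targeted skill.
; A per-tick camera line trace stores the aim point, outlines the targeted BP_AI through custom depth and animates the HUD crosshair color.
; Q toggles a decal at the aim point if MP and cooldown allow.
; Attack then plays a montage or spawns the skill's damage actor at the decal, using GameState skill data for cost and cooldown.
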(event Custom|ResetVariables
  ;[1 1 1] Attack
  (Variables|Default|SetisAttack false)
  (Variables|Default|SetSkillIndex 0))

(event Game|Damage|EventAnyDamage
  (params (Damage :type Float%20%28single-precision%29) (DamageType :type Damage%20Type%20Object%20Reference) (InstigatedBy :type Controller%20Object%20Reference) (DamageCauser :type Actor%20Object%20Reference))
  ;[1 1 1] HPChange
  (Variables|Default|SetCurrHP (Math|Float|Clamp(Float) (- (Variables|Default|GetCurrHP) Damage) 0.0 (Variables|Default|GetMaxHP))))

(event EventTick
  (params (DeltaSeconds :type Float%20%28single-precision%29))
  ;[1 1 1] CreateCrosshairAndSetRender
  (bind (_returnvalue _location _hitactor) (CallFunction|LineTraceTick))
  (if _returnvalue
    (Variables|Default|SetHitLocation _location)
    (bind _asbp_ai (Utilities|Casting|CastToBP_AI _hitactor)
      (:then
        (Utilities|IsValid (Variables|Default|GetAIActor)
          (:Is%20Valid
            (if (not (== (Variables|Default|GetAIActor) _asbp_ai))
              (CallFunction|SetRenderDepth false)
              (Variables|Default|SetAIActor _asbp_ai :!label _label)
              (CallFunction|SetRenderDepth true)
              (Utilities|FlowControl|Sequence
                (:then_0
                  (Utilities|FlowControl|DoOnce false :!label _label_2
                    (:Completed
                      (Default|CrosshairChangeColor (CallFunction|GetMainUI) "Forward"))))
                (:then_1
                  (goto _label_4 Reset)))))
          (:Is%20Not%20Valid
            (goto _label))))
      (:CastFailed
        (CallFunction|SetRenderDepth false :!label _label_3)
        (Variables|Default|SetAIActor 0)
        (Utilities|FlowControl|Sequence
          (:then_0
            ;;[1 1 1] 防止动画被重复触发
            (Utilities|FlowControl|DoOnce false :!label _label_4
              (:Completed
                (Default|CrosshairChangeColor (CallFunction|GetMainUI) "Reverse"))))
          (:then_1
            (goto _label_2 Reset)))))
    (else
      (Variables|Default|SetHitLocation "0.000000,0.000000, 0")
      (goto _label_3))))

(event Input|ActionEvents|InputActionAttack
  (params (Key :type Key%20Structure :default "None"))
  (bind _decalactor (Variables|Default|GetDecalActor))
  (bind _returnvalue (Transformation|GetActorLocation _decalactor))
  ;[1 1 1] Attack
  ;;[1 1 1] 鼠标左键
  (:Pressed
    (if (not (Variables|Default|GetisInSkillAEmitter))
      (if (not (Variables|Default|GetisAttack))
        (Variables|Default|SetisAttack true)
        (switch int (Variables|Default|GetSkillIndex)
          (:0
            (Animation|PlayAnimMontage "/Game/ThirdGame/Character/Animations/AnimMontage_NorAttack.AnimMontage_NorAttack" 1.0 "None"))
          (:1
            (Variables|Default|SetisInSkiilACoolDownTime true)
            (CallFunction|CallCDTimelimit)
            (Variables|Default|SetCurrentMP (- (Variables|Default|GetCurrentMP) (.MP (Utilities|Struct|BreakStruct_SkillInfo (CallFunction|SkillInfoFunc)))))
            (Variables|Default|SetisInSkillAEmitter true)
            (bind _returnvalue_2 (Game|SpawnActorfromClass "/Game/ThirdGame/Blueprints/BP_DamegedActor.BP_DamegedActor_C" (Math|Transform|MakeTransform _returnvalue "0, 0, 0" "1.000000,1.000000,1.000000") "Undefined" 0 0))
            (Development|PrintString (Utilities|String|ToString(Vector) _returnvalue))
            (Variables|Default|SetisInSkillAEmitter false)
            ;;[1 1 1] 举个例子
            ;; 假设技能CD是5秒：
            ;; 技能动画时长：1.67s
            ;; 实际需要额外等待的CD时间：5 - 1.67 = 3.33s
            ;; 总时间：1.67s(动画) + 3.33s(额外CD) = 5s(总CD)
            (Utilities|FlowControl|Delay (- (.CDTime (Utilities|Struct|BreakStruct_SkillInfo (CallFunction|SkillInfoFunc))) 1.67))
            (Variables|Default|SetisInSkiilACoolDownTime false)))))))

(event Input|ActionEvents|InputActionSkiiA
  (params (Key :type Key%20Structure :default "None"))
  ;[1 1 1] 按Q
  (:Pressed
    (if (not (Variables|Default|GetisAttack))
      (if (not (Class|AnimInstance|IsAnyMontagePlaying (Components|SkeletalMesh|GetAnimInstance (Variables|Character|GetMesh))))
        (if (> (Variables|Default|GetCurrentMP) (.MP (Utilities|Struct|BreakStruct_SkillInfo (CallFunction|SkillInfoFunc))))
          (if (not (Variables|Default|GetisInSkiilACoolDownTime))
            (if (!= (Variables|Default|GetSkillIndex) 1)
              ;[1 1 1] 开始技能时间，但是这个时候用户可能会点一次Q，skillIndex变成了0,
              (Variables|Default|SetSkillIndex 1)
              (bind _returnvalue (Game|SpawnActorfromClass "/Game/ThirdGame/Blueprints/BP_DecalActor.BP_DecalActor_C" (Math|Transform|MakeTransform (Variables|Default|GetHitLocation) "0, 0, 0" "1.000000,1.000000,1.000000") "Undefined" 0 0))
              (Variables|Default|SetDecalActor _returnvalue)
              (else
                ;[1 1 1] 不清楚 应该是因为有个状态的时候index可能是怕是2 3 4 什么数
                (Variables|Default|SetSkillIndex 0)
                ;[1 1 1] 为了按Q后松手 然后决定是否释放SkillA的技能
                (Actor|DestroyActor (Variables|Default|GetDecalActor))))))))))

(event Input|AxisEvents|InputAxisMoveForward
  (params (AxisValue :type Float%20%28single-precision%29))
  ;[1 1 1] Movement
  (Pawn|Input|AddMovementInput (Math|Vector|GetForwardVector (Math|Rotator|MakeRotator 0.0 0.0 (.Yaw (Math|Rotator|BreakRotator (Pawn|GetControlRotation :!class /Script/Engine.Pawn))))) AxisValue false))

(event Input|AxisEvents|InputAxisMoveRight
  (params (AxisValue :type Float%20%28single-precision%29))
  ;[1 1 1] Movement
  (Pawn|Input|AddMovementInput (Math|Vector|GetRightVector (Math|Rotator|MakeRotator 0.0 0.0 (.Yaw (Math|Rotator|BreakRotator (Pawn|GetControlRotation :!class /Script/Engine.Pawn))))) AxisValue false))

(event Input|AxisEvents|InputAxisTurnRight
  (params (AxisValue :type Float%20%28single-precision%29))
  ;[1 1 1] Movement
  (Pawn|Input|AddControllerYawInput AxisValue))

(event Input|AxisEvents|InputAxisTurnUp
  (params (AxisValue :type Float%20%28single-precision%29))
  ;[1 1 1] Movement
  (Pawn|Input|AddControllerPitchInput AxisValue))

(fn ConstructionScript)

(fn CallCDTimelimit
  (Default|CallCDTimeLimit (Utilities|Array|Get(acopy) (Variables|/Game/ThirdGame/UI/BP_MainUI.BP_MainUI_C|GetSkillUI (Variables|/Game/ThirdGame/GameModeBase/BP_HUD.BP_HUD_C|GetMainUI (.AsBP%20HUD (Utilities|Casting|CastToBP_HUD (HUD|GetHUD (Game|GetPlayerController 0)))))) (- (Variables|Default|GetSkillIndex) 1))))

(fn SkillInfoFunc
  (params (SkillIndex :type Integer))
  (return (Utilities|Array|Get(acopy) (.Skill (Utilities|Struct|BreakStruct_PlayerInfo (Utilities|Array|Get(acopy) (Variables|/Game/ThirdGame/GameModeBase/BP_GameStateBase.BP_GameStateBase_C|GetAllPlayersInfo (.AsBP%20Game%20State%20Base (Utilities|Casting|CastToBP_GameStateBase (Game|GetGameState)))) (Variables|Default|GetPlayerIndex)))) SkillIndex)))

(fn SetRenderDepth
  (params (isRender :type Boolean))
  ;[1 1 1] notvalid的时候怎么取消render?
  (Utilities|IsValid (Variables|Default|GetAIActor)
    (:Is%20Valid
      (Utilities|FlowControl|Sequence
        (:then_0
          (for _array_element (Actor|GetComponentsByClass (Variables|Default|GetAIActor) "/Script/Engine.StaticMeshComponent")
            (Rendering|SetRenderCustomDepth _array_element isRender)))
        (:then_1
          (for _array_element_2 (Actor|GetComponentsByClass (Variables|Default|GetAIActor) "/Script/Engine.SkeletalMeshComponent")
            (Rendering|SetRenderCustomDepth _array_element_2 isRender))))
      (if (not true)
        (Variables|Default|SetAIActor 0)))))

(fn LineTraceTick
  (bind _returnvalue (Game|GetPlayerCameraManager 0))
  (bind _returnvalue_2 (Transformation|GetActorLocation _returnvalue))
  (bind (_outhit _returnvalue_3) (Collision|LineTraceByChannel _returnvalue_2 (+ _returnvalue_2 (* (Transformation|GetActorForwardVector _returnvalue) 1e+03)) "TraceTypeQuery1" false 0 "None"))
  (return _returnvalue_3 (.Location (Collision|BreakHitResult _outhit)) (.HitActor (Collision|BreakHitResult _outhit))))

(fn SetAIRenderDepthEntire
  (params (TransAIActor :type BP%20AI%20Object%20Reference))
  (Utilities|IsValid (Variables|Default|GetAIActor)
    (:Is%20Valid
      (if (not (== (Variables|Default|GetAIActor) TransAIActor))
        (CallFunction|SetRenderDepth false)
        (Variables|Default|SetAIActor TransAIActor :!label _label)
        (CallFunction|SetRenderDepth true)))
    (:Is%20Not%20Valid
      (goto _label))))

(fn GetMainUI
  (return (Variables|/Game/ThirdGame/GameModeBase/BP_HUD.BP_HUD_C|GetMainUI (.AsBP%20HUD (Utilities|Casting|CastToBP_HUD (HUD|GetHUD (Game|GetPlayerController 0)))))))