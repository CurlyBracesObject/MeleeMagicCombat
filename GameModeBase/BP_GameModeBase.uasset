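; Game mode that tracks monster kills and respawns Kobold enemies until three have been killed.
; ReportEnemyKilled increments and prints the kill count, then below the limit spawns BP_AI_Kobold at the BP_FixedSpawnLocation actor.
; It also advances MonsterIndex and calls SetMonsterType on the stored AIActor reference, which is not updated to the new spawn.
; A disconnected zero-HP check on AIActor never runs.
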(event Custom|ReportEnemyKilled
  (bind _aiactor (Variables|Default|GetAIActor))
  (Math|Integer|IncrementInt (Variables|Default|GetKilledMonsterCount)
    (:%20%20
      (Development|PrintString (Utilities|String|ToString(Integer) (Variables|Default|GetKilledMonsterCount)))
      (if (< (Variables|Default|GetKilledMonsterCount) 3)
        (Math|Integer|IncrementInt (Variables|/Game/ThirdGame/Enemy/BP_AI.BP_AI_C|GetMonsterIndex _aiactor)
          (:%20%20
            (bind _returnvalue (Actor|GetActorOfClass "/Game/ThirdGame/Blueprints/BP_FixedSpawnLocation.BP_FixedSpawnLocation_C"))
            (Game|SpawnActorfromClass "/Game/ThirdGame/Enemy/Kobold/BP_AI_Kobold.BP_AI_Kobold_C" (Transformation|GetActorTransform _returnvalue) "Undefined" 0 0)
            (Default|SetMonsterType _aiactor)))))))

(fn ConstructionScript)