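; BP_PC is a player controller that moves the player from a start pawn into gameplay in the FrozenCove level.
; On BeginPlay it caches the initial BP_StartPawn.
; LevelChangeAndAfterLogic loads FrozenCove as a blocking stream level, then shows the main UI through BP_HUD.
; It then spawns a BP_Character at the PlayerStart found in the world, possesses it and destroys the start pawn.
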(event Custom|LevelChangeAndAfterLogic
  (Class|GameplayStatics|LoadStreamLevelbySoftObjectPtr "/Game/InfinityBladeIceLands/Maps/FrozenCove.FrozenCove" true true)
  (Utilities|FlowControl|Sequence
    (:then_0
      (Default|ShowMainUI (.AsBP%20HUD (Utilities|Casting|CastToBP_HUD (HUD|GetHUD)))))
    (:then_1
      (bind _returnvalue (Actor|GetActorOfClass "/Script/Engine.PlayerStart"))
      (bind _returnvalue_2 (Game|SpawnActorfromClass "/Game/ThirdGame/Character/BP_Character.BP_Character_C" (Transformation|GetActorTransform _returnvalue) "Undefined" 0 0))
      (Pawn|Possess _returnvalue_2)
      (Actor|DestroyActor (Variables|Default|GetStartPawn)))))

(event EventBeginPlay
  (Variables|Default|SetStartPawn (.AsBP%20Start%20Pawn (Utilities|Casting|CastToBP_StartPawn (Game|Player|GetPlayerPawn 0)))))

(fn ConstructionScript)